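; BP_SwatController is the player controller for the BP_Swat character, turning Enhanced Input actions into movement, camera and combat commands.
; On BeginPlay it adds the IMC_Swat mapping context and caches the possessed Swat pawn.
; Movement follows control yaw, while sprint, walk, aim and fire are forwarded to the pawn.
; Sprint is blocked while aiming, aim uses a DoOnce and checks falling, and firing requires aiming, branching on semi-auto or auto mode.
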(event Input|EnhancedActionEvents|EnhancedInputActionIA_MoveSwat
  (params (ActionValue :type Vector%202D%20Structure) (ElapsedSeconds :type Float%20%28double-precision%29) (TriggeredSeconds :type Float%20%28double-precision%29) (InputAction :type Input%20Action%20Object%20Reference :default "/Game/Assets/Inputs/IA_MoveSwat.IA_MoveSwat"))
  (bind _returnvalue (Pawn|GetControlRotation :!class /Script/Engine.Controller))
  (bind _swatplayer (Variables|Default|GetSwatPlayer))
  (bind _returnvalue_2 (Math|Rotator|MakeRotator 0.0 0.0 (.yaw _returnvalue)))
  ;[0.15 0.15 0.15 0.5] Player RPG Movement
  (Pawn|Input|AddMovementInput _swatplayer (Math|Vector|GetForwardVector _returnvalue_2) (.x ActionValue) false)
  (Pawn|Input|AddMovementInput _swatplayer (Math|Vector|GetRightVector _returnvalue_2) (.y ActionValue) false))

(event Input|EnhancedActionEvents|EnhancedInputActionIA_RotateSwat
  (params (ActionValue :type Vector%202D%20Structure) (ElapsedSeconds :type Float%20%28double-precision%29) (TriggeredSeconds :type Float%20%28double-precision%29) (InputAction :type Input%20Action%20Object%20Reference :default "/Game/Assets/Inputs/IA_RotateSwat.IA_RotateSwat"))
  ;[0.15 0.15 0.15 0.5] Player Rotation
  (Class|PlayerController|AddPitchInput (.y ActionValue))
  (Class|PlayerController|AddYawInput (.x ActionValue)))

(event Input|EnhancedActionEvents|EnhancedInputActionIA_SprintSwat
  (params (ActionValue :type Boolean) (ElapsedSeconds :type Float%20%28double-precision%29) (TriggeredSeconds :type Float%20%28double-precision%29) (InputAction :type Input%20Action%20Object%20Reference :default "/Game/Assets/Inputs/IA_SprintSwat.IA_SprintSwat"))
  (bind _swatplayer (Variables|Default|GetSwatPlayer))
  ;[0.15 0.15 0.15 0.5] Player Sprint / Walk
  (:Triggered
    (if (not (Variables|/Game/Blueprints/BP_Swat.BP_Swat_C|GetAiming? _swatplayer))
      (Default|Sprint _swatplayer true)))
  (:Completed
    (Default|Sprint _swatplayer false)))

(event Input|EnhancedActionEvents|EnhancedInputActionIA_WalkSwat
  (params (ActionValue :type Boolean) (ElapsedSeconds :type Float%20%28double-precision%29) (TriggeredSeconds :type Float%20%28double-precision%29) (InputAction :type Input%20Action%20Object%20Reference :default "/Game/Assets/Inputs/IA_WalkSwat.IA_WalkSwat"))
  (bind _swatplayer (Variables|Default|GetSwatPlayer))
  ;[0.15 0.15 0.15 0.5] Player Sprint / Walk
  (:Triggered
    (Default|Walk _swatplayer true))
  (:Completed
    (Default|Walk _swatplayer false)))

(event Input|EnhancedActionEvents|EnhancedInputActionIA_Fire
  (params (ActionValue :type Boolean) (ElapsedSeconds :type Float%20%28double-precision%29) (TriggeredSeconds :type Float%20%28double-precision%29) (InputAction :type Input%20Action%20Object%20Reference :default "/Game/Assets/Inputs/IA_Fire.IA_Fire"))
  (bind _swatplayer (Variables|Default|GetSwatPlayer))
  (bind _firemode (Variables|/Game/Blueprints/BP_Swat.BP_Swat_C|GetFiremode _swatplayer))
  (:Started
    (if (Variables|/Game/Blueprints/BP_Swat.BP_Swat_C|GetAiming? _swatplayer)
      (switch Utilities|FlowControl|Switch|SwitchonE_Firemode _firemode
        (:NewEnumerator0
          (Default|Fire _swatplayer))
        (:NewEnumerator1
          (Default|AutoFire _swatplayer true)))))
  (:Completed
    (switch Utilities|FlowControl|Switch|SwitchonE_Firemode _firemode
      (:NewEnumerator1
        (Default|AutoFire _swatplayer false)))))

(event Input|EnhancedActionEvents|EnhancedInputActionIA_Aim
  (params (ActionValue :type Boolean) (ElapsedSeconds :type Float%20%28double-precision%29) (TriggeredSeconds :type Float%20%28double-precision%29) (InputAction :type Input%20Action%20Object%20Reference :default "/Game/Assets/Inputs/IA_Aim.IA_Aim"))
  (bind _swatplayer (Variables|Default|GetSwatPlayer))
  ;[0.15 0.15 0.15 0.5] Player Aim
  (:Triggered
    (if (Variables|/Game/Blueprints/BP_Swat.BP_Swat_C|GetFalling _swatplayer)
      (Default|AimorNot _swatplayer false)
      (goto _label Reset)
      (else
        (Utilities|FlowControl|DoOnce false :!label _label
          (:Completed
            (if (Variables|/Game/Blueprints/BP_Swat.BP_Swat_C|GetSprint? _swatplayer)
              (Default|Sprint _swatplayer false))
            (Default|AimorNot _swatplayer true))))))
  (:Completed
    (Default|AimorNot _swatplayer false)
    (goto _label Reset)))

(event EventBeginPlay
  (Input|AddMappingContext (PlayerController|LocalPlayerSubsystems|GetEnhancedInputLocalPlayerSubsystem) "/Game/Assets/Inputs/IMC_Swat.IMC_Swat" 0 "(bIgnoreAllPressedKeysUntilRelease=True,bForceImmediately=False,bNotifyUserSettings=False)")
  (bind _asbp_swat (Utilities|Casting|CastToBP_Swat (Game|Player|GetPlayerPawn 0)))
  (Variables|Default|SetSwatPlayer _asbp_swat))

(event EventTick
  (params (DeltaSeconds :type Float%20%28single-precision%29)))

(fn ConstructionScript)