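; Generator actor that places a random selection of enemy spawners from an editable list of candidate points at game start.
; The construction script grows the list to MaxSPs if short and previews each point with a marker mesh and flattened meshes scaled to min/max spawn radius.
; BeginPlay shuffles the points, spawns EnemySPsEach BP_EnemySpawners, passes the spawner-to-point collection to BP_WaveManager, then destroys the preview meshes.
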(event EventBeginPlay
  (bind _sps (Variables|Default|GetSPs))
  (Utilities|Array|Shuffle _sps)
  (for _index (range 0 (- (Variables|Default|GetEnemySPsEach) 1))
    (bind _returnvalue (Game|SpawnActorfromClass "/Game/Blueprints/BP_EnemySpawner.BP_EnemySpawner_C" (Math|Transform|MakeTransform (Utilities|Array|Get(acopy) _sps _index) "0, 0, 0" "1.000000,1.000000,1.000000") "Undefined" "MultiplyWithRoot" 0 (Variables|Default|GetMinSPRange) (Variables|Default|GetMaxSPRange) 0))
    (Utilities|Array|Add (Variables|Default|GetSP%20and%20Gen%20Points) (Utilities|Struct|MakeST_SPAndGen _returnvalue (Utilities|Array|Get(acopy) _sps _index))))
  (bind _returnvalue_2 (Actor|GetActorOfClass "/Game/Blueprints/BP_WaveManager.BP_WaveManager_C"))
  (Default|AllSpawnerPlaced _returnvalue_2 (Variables|Default|GetSP%20and%20Gen%20Points))
  (for _array_element (Variables|Default|GetSigns)
    (Components|DestroyComponent _array_element)))

(event Collision|EventActorBeginOverlap
  (params (OtherActor :type Actor%20Object%20Reference)))

(event EventTick
  (params (DeltaSeconds :type Float%20%28single-precision%29)))

(fn ConstructionScript
  (bind _maxsprange (Variables|Default|GetMaxSPRange))
  (bind _minsprange (Variables|Default|GetMinSPRange))
  (bind _maxsps (Variables|Default|GetMaxSPs))
  (bind _sps (Variables|Default|GetSPs))
  (bind _returnvalue (/ _maxsprange 5e+01))
  (bind _returnvalue_2 (/ _minsprange 5e+01))
  (if (> _maxsps (Utilities|Array|Length (Variables|Default|GetSPs)))
    (Utilities|Array|Resize _sps _maxsps)
    (bind _returnvalue_3 (AddComponent|AddStaticMeshComponent false (Math|Transform|MakeTransform (stale _array_element) "0, 0, 0" "1.000000,1.000000,1.000000") :!label _label))
    (Utilities|Array|Add (Variables|Default|GetSigns) _returnvalue_3)
    (bind _returnvalue_4 (AddComponent|AddStaticMeshComponent false (Math|Transform|MakeTransform (stale _array_element) "0, 0, 0" (Math|Vector|MakeVector _returnvalue_2 _returnvalue_2 0.06))))
    (Utilities|Array|Add (Variables|Default|GetSigns) _returnvalue_4)
    (bind _returnvalue_5 (AddComponent|AddStaticMeshComponent false (Math|Transform|MakeTransform (stale _array_element) "0, 0, 0" (Math|Vector|MakeVector _returnvalue _returnvalue 0.05))))
    (Utilities|Array|Add (Variables|Default|GetSigns) _returnvalue_5)
    (else
      (for _array_element _sps
        (goto _label)))))