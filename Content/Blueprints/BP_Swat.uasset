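; Player SWAT character for a third-person wave shooter, handling aiming, M4 shooting and reload, damage with knockback, and death that reloads the level.
; A camera trace with movement-dependent spread aims BP_Bullet projectiles from the muzzle, or applies instant hits up close.
; Montage notifies drive magazine swaps during reload.
; Tick updates spread, speed, predicted-path landing detection and an arrow toward the current wave's generator.
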(event Custom|Fire
  (bind _self self)
  (bind _camtps (Variables|Default|GetCamTPS))
  (bind _shelllaunch_ (Variables|Default|GetShellLaunch%20))
  (bind _muzzle (Variables|Default|GetMuzzle))
  (bind _returnvalue (Transformation|GetWorldTransform _muzzle))
  (bind _returnvalue_2 (Transformation|GetWorldLocation _camtps))
  ;[0.15 0.05212 0.05212 0.5 118] Shooting Logic
  (if (Math|Conversions|ToBoolean(Integer) (Variables|Default|GetAmmunition))
    (Animation|Montage|PlayMontage (Variables|Character|GetMesh) "/Game/Assets/Characters/Swat/Animations/AM_Shooting.AM_Shooting" 1.0 0.0 "Fire"
      (:then
        (Niagara|SpawnSystemAttached "/Game/Blueprints/Niagara/NS_MuzzleFlash.NS_MuzzleFlash" (Variables|Default|GetMuzzleArrow) "None" "0, 0, 0" "0, 0, 0" "KeepRelativeOffset" true)
        (Variables|Default|SetTimeElapsedAfterShot (Utilities|Time|GetTimeSeconds))
        (bind (_outhit _returnvalue_3) (Collision|LineTraceByChannel _returnvalue_2 (+ _returnvalue_2 (* (Math|Random|RandomUnitVectorinConeinDegrees (Math|Vector|GetForwardVector _camtps) (* (Math|Float|Max(Float) (- (Variables|Default|GetCurrentSpread) (Variables|Default|GetMinSpread)) 0.0) (Variables|Default|GetSpreadRadius))) 9e+04)) "TraceTypeQuery3" false 0 "None"))
        (if _returnvalue_3
          (if (< (.Distance (Collision|BreakHitResult _outhit)) 3e+02)
            (Game|SpawnActorfromClass "/Game/Blueprints/BP_Bullet.BP_Bullet_C" (Math|Conversions|ToTransform(Vector) (.ImpactPoint (Collision|BreakHitResult _outhit))) "Undefined" "MultiplyWithRoot" 0 "0.000000,0.000000,0.000000" true _outhit _self)
            (else
              (Game|SpawnActorfromClass :Class "/Game/Blueprints/BP_Bullet.BP_Bullet_C" :SpawnTransform _returnvalue :CollisionHandlingOverride "Undefined" :TransformScaleMethod "MultiplyWithRoot" :Velocity (* (Math|Vector|Normalize (- (.Location (Collision|BreakHitResult _outhit)) (Transformation|GetWorldLocation _muzzle))) 9e+04) :Instigator _self)))
          (else
            (Game|SpawnActorfromClass :Class "/Game/Blueprints/BP_Bullet.BP_Bullet_C" :SpawnTransform _returnvalue :CollisionHandlingOverride "Undefined" :TransformScaleMethod "MultiplyWithRoot" :Velocity (* (Math|Random|RandomUnitVectorinConeinDegrees (Math|Vector|GetForwardVector _camtps) (* (Math|Float|Max(Float) (- (Variables|Default|GetCurrentSpread) (Variables|Default|GetMinSpread)) 0.0) (Variables|Default|GetSpreadRadius))) 9e+04) :Instigator _self)))
        (Audio|PlaySoundatLocation "/Game/Assets/Sounds/Weapon/M4_FireCue.M4_FireCue" (Transformation|GetWorldLocation (Variables|Default|GetMuzzle)) "0, 0, 0" 1.0 1.0 0.0 0 0 0 0)
        (Variables|Default|SetAmmunition (- (Variables|Default|GetAmmunition) 1))
        (Game|SpawnActorfromClass "/Game/Blueprints/BP_DroppedShell.BP_DroppedShell_C" (Math|Transform|MakeTransform (Transformation|GetWorldLocation _shelllaunch_) (Transformation|GetWorldRotation _shelllaunch_)) "Undefined" "MultiplyWithRoot" 0 (Math|Vector|GetForwardVector _shelllaunch_) 0)
        (bind _output_get (Variables|Default|SetCurrentSpread (* (Variables|Default|GetCurrentSpread) (Variables|Default|GetSpreadIncrement))))
        (if (> _output_get 1e+01)
          (Variables|Default|SetCurrentSpread 1e+01))))
    (else
      (CallFunction|StopFire)
      (Utilities|FlowControl|DoOnce false
        (:Completed
          (Audio|PlaySound2D "/Game/Assets/Sounds/Weapon/M4_Empty.M4_Empty" 1.0 1.0 0.0 0 0))))))

(event Custom|AutoFire
  (params (On :type Boolean))
  ;[0.15 0.05212 0.05212 0.5 118] Shooting Logic
  ;;[0.15 0.15 0.15 0.5 50] AutoFire
  (if On
    (Utilities|Time|UnpauseTimerbyHandle (Variables|Default|GetAutoFireTimer))
    (else
      (Utilities|Time|PauseTimerbyHandle (Variables|Default|GetAutoFireTimer)))))

(event Custom|ShutdownUI
  (Widget|RemovefromParent (Variables|Default|GetCrosshairUI)))

(event Custom|Landed
  ;[0.15 0.15 0.15 0.5 41] On Air & Jump
  (CallFunction|LandingDeceleration)
  (Variables|Default|SetJumped false)
  (Utilities|FlowControl|DoOnce false) ; enters at Reset
)

(event Custom|Reload
  (bind _magazine (Variables|Default|GetMagazine))
  (bind _mesh (Variables|Character|GetMesh))
  ;[0.15 0.05212 0.05212 0.5 118] Shooting Logic
  ;;[0.15 0.15 0.15 0.5 68] Reload
  (Utilities|FlowControl|DoOnce false :!label _label
    (:Completed
      (Variables|Default|SetInterpReload false)
      (Variables|Default|SetReloading true)
      (CallFunction|StopFire)
      (bind _notifyname (Animation|Montage|PlayMontage _mesh "/Game/Assets/Characters/Swat/Animations/AM_Shooting.AM_Shooting" 1.2 0.0 "Reload")
        (:then
          (Transformation|AttachComponentToComponent (Variables|Default|GetM4) _mesh "RifleSocketAim" "KeepRelative" "KeepRelative" "KeepRelative" true))
        (:OnBlendOut
          (Variables|Default|SetReloading false)
          (Animation|Montage|PlayMontage _mesh "/Game/Assets/Characters/Swat/Animations/AM_Shooting.AM_Shooting" 1.0 0.0 "Aim"
            (:then
              (if (and (Variables|Default|GetLMouseHold) (Utilities|Enum|Equal(Enum) (Variables|Default|GetFiremode) "NewEnumerator1"))
                (Utilities|Time|UnpauseTimerbyHandle (Variables|Default|GetAutoFireTimer))
                (goto _label Reset)
                (else
                  (goto _label Reset))))))
        (:OnNotifyBegin
          (switch name _notifyname
            (:Detach
              (Transformation|AttachComponentToComponent (Variables|Default|GetMagazine) (Variables|Character|GetMesh) "MagazineSocket" "SnapToTarget" "SnapToTarget" "KeepWorld" true)
              (Audio|PlaySound2D "/Game/Assets/Sounds/Weapon/M4_ReloadFirst.M4_ReloadFirst" 1.0 1.0 0.0 0 0))
            (:Throw
              (Rendering|SetVisibility _magazine false false)
              (Game|SpawnActorfromClass "/Game/Blueprints/BP_DroppedMag.BP_DroppedMag_C" (Transformation|GetWorldTransform _magazine) "Undefined" "MultiplyWithRoot" 0 0))
            (:Get
              (Rendering|SetVisibility _magazine true false)
              (Transformation|AttachComponentToComponent (Variables|Default|GetMagazine) (Variables|Character|GetMesh) "MagazineSocket" "KeepRelative" "KeepRelative" "KeepWorld" true))
            (:Attach
              (Transformation|AttachComponentToComponent (Variables|Default|GetMagazine) (Variables|Default|GetM4) "Magazine" "KeepRelative" "KeepRelative" "KeepWorld" true)
              (Audio|PlaySound2D "/Game/Assets/Sounds/Weapon/M4_ReloadMid.M4_ReloadMid" 1.0 1.0 0.0 0 0)
              (Variables|Default|SetAmmunition (Variables|Default|GetMagazineCap)))
            (:Click
              (Variables|Default|SetInterpReload true)
              (Audio|PlaySound2D "/Game/Assets/Sounds/Weapon/M4_ReloadLast.M4_ReloadLast" 1.0 1.0 0.0 0 0)
              (if (not (Variables|Default|GetAiming))
                (Transformation|AttachComponentToComponent (Variables|Default|GetM4) (Variables|Character|GetMesh) "RifleSocketMove" "KeepRelative" "KeepRelative" "KeepRelative" true)))))))))

(event Custom|Dead
  (params (BackAttack :type Boolean))
  (bind _mesh (Variables|Character|GetMesh))
  ;[0.15 0.15 0.15 0.5 36] Damaged
  (Audio|PlaySound2D "/Game/Assets/Sounds/Swat/SwatDeathCue.SwatDeathCue" 1.0 1.0 0.0 0 0)
  (bind _asbp_swat_controller (Utilities|Casting|CastToBP_SwatController (Game|GetPlayerController 0)))
  (Default|OnDeadEvent _asbp_swat_controller)
  (Input|DisableInput 0)
  (Utilities|Time|ClearandInvalidateTimerbyHandle (Variables|Default|GetAutoFireTimer))
  (Components|Movement|StopMovementImmediately (Variables|Character|GetCharacterMovement))
  (if BackAttack
    (Animation|Montage|PlayMontage _mesh "/Game/Assets/Characters/Swat/Animations/AM_Death.AM_Death" 1.0 0.0 "Forward"
      (:OnNotifyBegin
        _))
    (else
      (Animation|Montage|PlayMontage _mesh "/Game/Assets/Characters/Swat/Animations/AM_Death.AM_Death" 1.0 0.0 "Back"
        (:OnNotifyBegin
          _))))
  (bind _returnvalue (Game|GetCurrentLevelName true))
  (Game|OpenLevel(byName) (Utilities|String|StringToName _returnvalue)))

(event Custom|StopFire
  ;[0.15 0.05212 0.05212 0.5 118] Shooting Logic
  ;;[0.15 0.15 0.15 0.5 50] AutoFire
  (Utilities|Time|PauseTimerbyHandle (Variables|Default|GetAutoFireTimer)))

(event Custom|EmptySoundReset
  ;[0.15 0.05212 0.05212 0.5 118] Shooting Logic
  (Utilities|FlowControl|DoOnce false) ; enters at Reset
)

(event Custom|AfterGeneratorSpawned
  (params (WaveManager :type BP%20Wave%20Manager%20Object%20Reference))
  (bind _self self)
  ;[0.15 0.15 0.15 0.5] UI
  (bind _returnvalue (UserInterface|CreateWidget "/Game/Blueprints/UI/InGameUI.InGameUI_C" 0 _self WaveManager))
  (bind _output_get (Variables|Default|SetInGameUI _returnvalue))
  (UserInterface|Viewport|AddtoViewport _output_get 0)
  (bind _returnvalue_2 (UserInterface|CreateWidget "/Game/Blueprints/UI/CrosshairUI.CrosshairUI_C" 0 _self))
  (bind _output_get_2 (Variables|Default|SetCrosshairUI _returnvalue_2))
  (UserInterface|Viewport|AddtoViewport _output_get_2 0)
  (Widget|SetVisibility _output_get_2 "Hidden")
  (bind _returnvalue_3 (UserInterface|CreateWidget "/Game/Blueprints/UI/InteractUI.InteractUI_C"))
  (bind _output_get_3 (Variables|Default|SetInteractUI _returnvalue_3))
  (UserInterface|Viewport|AddtoViewport _output_get_3 0))

(event Custom|Set%20Nearby%20Generator
  (params (Generator :type BP%20Generator%20Object%20Reference))
  ;[0.15 0.15 0.15 0.5] InteractUI
  (bind _text (Class|InteractInterface|GetInteractText(Message) Generator))
  (Default|SetGenerator (Variables|Default|GetInteractUI) _text Generator))

(event Custom|Unset%20Nearby%20Generator
  ;[0.15 0.15 0.15 0.5] InteractUI
  (Default|UnsetGenerator (Variables|Default|GetInteractUI)))

(event Input|EnhancedActionEvents|EnhancedInputActionIA_JumpSwat
  (params (ActionValue :type Boolean) (ElapsedSeconds :type Float%20%28double-precision%29) (TriggeredSeconds :type Float%20%28double-precision%29) (InputAction :type Input%20Action%20Object%20Reference :default "/Game/Assets/Inputs/IA_JumpSwat.IA_JumpSwat"))
  ;[0.15 0.15 0.15 0.5 41] On Air & Jump
  (Utilities|FlowControl|DoOnce false
    (:Completed
      (Variables|Default|SetJumped true))))

(event EventBeginPlay
  ;[0.15 0.15 0.15 0.5] Autofire Timer
  (Variables|Default|SetSPR (/ 6e+01 (Variables|Default|GetRPM)))
  (bind _returnvalue (Utilities|Time|SetTimerbyEvent (EventDispatchers|CreateEvent :!event Custom|Fire) (Variables|Default|GetSPR) true))
  (bind _output_get (Variables|Default|SetAutoFireTimer _returnvalue))
  (Utilities|Time|PauseTimerbyHandle _output_get))

(event Collision|EventActorBeginOverlap
  (params (OtherActor :type Actor%20Object%20Reference)))

(event EventTick
  (params (DeltaSeconds :type Float%20%28single-precision%29))
  (CallFunction|FindGenerator)
  (CallFunction|RecoverSpread DeltaSeconds)
  (CallFunction|SetForwardandRightSpeed)
  (CallFunction|WalkDeceleration DeltaSeconds)
  (if (Variables|Default|GetInterpReload)
    (Variables|Default|SetReloadBlendWeight (Math|Interpolation|FInterpTo (Variables|Default|GetReloadBlendWeight) 0.0 DeltaSeconds 4.0))
    (else
      (Variables|Default|SetReloadBlendWeight 1.0)))
  ;[0.15 0.15 0.15 0.5 41] On Air & Jump
  (bind _output_get (Variables|Default|SetFalling (AI|Components|NavMovement|IsFalling (Variables|Character|GetCharacterMovement))))
  (Variables|Default|SetLand (CallFunction|ReadytoLand?))
  (if (and (Variables|Default|GetJumped) _output_get)
    (Variables|Default|SetJumped false)
    (Utilities|FlowControl|DoOnce false) ; enters at Reset
  ))

(event EventEndPlay
  (params (EndPlayReason :type EEndPlayReason%20Enum :default "Destroyed"))
  (Widget|RemovefromParent (Variables|Default|GetCrosshairUI)))

(event EventApplyKnockback
  (params (Damage%20Causer :type Actor%20Object%20Reference) (Strength :type Float%20%28double-precision%29))
  ;[0.15 0.15 0.15 0.5 36] Damaged
  ;;[0.15 0.15 0.15 0.5 27] Knockback
  (Character|LaunchCharacter (+ (* Strength (Math|Vector|Normalize (- (Transformation|GetActorLocation) (Transformation|GetActorLocation Damage%20Causer)))) "0.000000,0.000000,20.000000") false false))

(event Game|Damage|EventAnyDamage
  (params (Damage :type Float%20%28single-precision%29) (DamageType :type Damage%20Type%20Object%20Reference) (InstigatedBy :type Controller%20Object%20Reference) (DamageCauser :type Actor%20Object%20Reference))
  (bind _healthcomponent (Variables|Default|GetHealthComponent))
  ;[0.15 0.15 0.15 0.5 36] Damaged
  (Default|GetDamage _healthcomponent Damage)
  (if (Variables|/Game/Blueprints/Component/HealthComponent.HealthComponent_C|GetIsDead? _healthcomponent)
    (Utilities|FlowControl|DoOnce false
      (:Completed
        (CallFunction|Dead (< (Math|Vector|DotProduct (Transformation|GetActorForwardVector) (Math|Vector|Normalize (- (Transformation|GetActorLocation) (Transformation|GetActorLocation DamageCauser)))) 0.0))))
    (else
      (Audio|PlaySound2D "/Game/Assets/Sounds/Swat/SwatHurtCue.SwatHurtCue" 1.0 1.0 0.0 0 0)
      (bind _strength (Class|KnockbackInteface|KnockbackStrength(Message) DamageCauser))
      (CallFunction|ApplyKnockback DamageCauser _strength))))

(event Input|KeyboardEvents|V
  (params (Key :type Key%20Structure :default "None"))
  ;[0.15 0.05212 0.05212 0.5 118] Shooting Logic
  (:Pressed
    (CallFunction|StopFire)
    (CallFunction|ToggleFiremode)))

(event Input|KeyboardEvents|E
  (params (Key :type Key%20Structure :default "None"))
  ;[0.15 0.15 0.15 0.5] InteractUI
  (:Pressed
    (Default|ActiveGenerator (Variables|Default|GetInteractUI))))

(fn ConstructionScript)

(fn Sprint
  (params (Sprint? :type Boolean))
  (bind _output_get (Variables|Default|SetSprinting Sprint?))
  (if _output_get
    (Variables|/Script/Engine.CharacterMovementComponent|SetMaxWalkSpeed (Variables|Character|GetCharacterMovement) 586.0)
    (Variables|Default|SetCurrentMaxSpeed 586.0)
    (else
      (Variables|Default|SetCurrentMaxSpeed 452.0))))

(fn Walk
  (params (Walk? :type Boolean))
  (bind _charactermovement (Variables|Character|GetCharacterMovement))
  (if Walk?
    (Variables|/Script/Engine.CharacterMovementComponent|SetMaxWalkSpeed _charactermovement 184.0)
    (else
      (Variables|/Script/Engine.CharacterMovementComponent|SetMaxWalkSpeed _charactermovement 452.0))))

(fn SetForwardandRightSpeed
  (bind _returnvalue (Transformation|GetVelocity))
  (bind _charactermovement (Variables|Character|GetCharacterMovement))
  (bind _velocity (Variables|/Script/Engine.MovementComponent|GetVelocity _charactermovement))
  (bind _returnvalue_2 (Math|Vector|VectorLength _velocity))
  ;[0.15 0.15 0.15 0.5 32] Calculate Forward/Right Speed
  (Variables|Default|SetSpeedRight (Math|Vector|DotProduct _returnvalue (Transformation|GetActorRightVector)))
  (Variables|Default|SetSpeedForward (Math|Vector|DotProduct _returnvalue (Transformation|GetActorForwardVector)))
  ;[0.15 0.1087 0.1285 0.5 32] Spread
  (if (<= _returnvalue_2 0.05)
    ;;[0.15 0.15 0.15 0.5] Stop
    (Variables|Default|SetMinSpread 0.6)
    (Variables|Default|SetSpreadIncrement 1.2)
    (Variables|Default|SetSpreadRecoverSpeed 2.5)
    (elif (<= _returnvalue_2 185.0)
      ;;[0.15 0.15 0.15 0.5] Walk
      (Variables|Default|SetMinSpread 0.7)
      (Variables|Default|SetSpreadIncrement 1.2)
      (Variables|Default|SetSpreadRecoverSpeed 2.4)
      (else
        ;;[0.15 0.15 0.15 0.5] Run/Sprint
        (Variables|Default|SetMinSpread 1.2)
        (Variables|Default|SetSpreadIncrement 1.4)
        (Variables|Default|SetSpreadRecoverSpeed 1.8)))))

(fn WalkDeceleration
  (params (DeltaTime :type Float%20%28double-precision%29))
  (bind _currentmaxspeed (Variables|Default|GetCurrentMaxSpeed))
  (bind _charactermovement (Variables|Character|GetCharacterMovement))
  ;[0.15 0.15 0.15 0.5] Set Max Walk Speed with Interpolation
  (if (< _currentmaxspeed (Variables|/Script/Engine.CharacterMovementComponent|GetMaxWalkSpeed _charactermovement))
    (Variables|/Script/Engine.CharacterMovementComponent|SetMaxWalkSpeed _charactermovement (Math|Interpolation|FInterpTo (Variables|/Script/Engine.CharacterMovementComponent|GetMaxWalkSpeed _charactermovement) _currentmaxspeed DeltaTime 8.0))))

(fn ReadytoLand?
  (if (Variables|Default|GetFalling)
    ;[0.15 0.15 0.15 0.5] Falling?
    (if (< (.z (Transformation|GetVelocity)) 0.0)
      ;[0.15 0.15 0.15 0.5] Near Ground?
      (bind _predictresult (Class|GameplayStatics|BlueprintPredictProjectilePathAdvanced (Utilities|Struct|MakePredictProjectilePathParams (- (Transformation|GetActorLocation) (Math|Vector|MakeVector 0.0 0.0 (Components|Capsule|GetScaledCapsuleHalfHeight (Variables|Collision|GetCapsuleComponent)))) (Transformation|GetVelocity) true 0.0 1.2 true "ECC_WorldStatic" "ObjectTypeQuery1" (Utilities|Array|MakeArray self) 4e+01 (Components|Movement|GetGravityZ (Variables|Character|GetCharacterMovement)) "None" 1.0 false)))
      (return (and (.bblockinghit (.hitresult _predictresult)) (<= (/ (+ (Math|Conversions|ToFloat(Integer) (Utilities|Array|LastIndex (.pathdata _predictresult))) (.time (.hitresult _predictresult))) 4e+01) 0.3)))
      (else
        _)))
  (return false))

(fn AimorNot
  (params (On :type Boolean))
  (bind _reloading (Variables|Default|GetReloading))
  (bind _m4 (Variables|Default|GetM4))
  (bind _charactermovement (Variables|Character|GetCharacterMovement))
  (bind _crosshairui (Variables|Default|GetCrosshairUI))
  (bind _mesh (Variables|Character|GetMesh))
  (bind _springarm (Variables|Default|GetSpringArm))
  (bind _camtps (Variables|Default|GetCamTPS))
  (if On
    (Variables|Default|SetAiming true)
    (Variables|/Script/Engine.SpringArmComponent|SetTargetArmLength _springarm 1e+02)
    (Variables|/Script/Engine.SpringArmComponent|SetbEnableCameraLag _springarm false)
    (Camera|SetFieldOfView _camtps 75.0)
    (Transformation|SetRelativeLocation _camtps "0.000000,50.000000,0.000000" false false)
    (Variables|/Script/Engine.CharacterMovementComponent|SetbOrientRotationToMovement _charactermovement false)
    (Variables|Default|SetbUseControllerRotationYaw true)
    (Transformation|AttachComponentToComponent _m4 _mesh "RifleSocketAim" "KeepRelative" "KeepRelative" "KeepRelative" true)
    (if _reloading
      _
      (else
        (Animation|PlayAnimMontage "/Game/Assets/Characters/Swat/Animations/AM_Shooting.AM_Shooting" 1.0 "Aim")
        (if (Variables|Default|GetLMouseHold)
          (Utilities|Time|UnpauseTimerbyHandle (Variables|Default|GetAutoFireTimer)))))
    (Utilities|IsValid _crosshairui
      (:Is%20Valid
        (Widget|SetVisibility _crosshairui "Visible")))
    (else
      (Variables|Default|SetAiming false)
      (CallFunction|AutoFire false)
      (Variables|/Script/Engine.SpringArmComponent|SetTargetArmLength _springarm 3e+02)
      (Variables|/Script/Engine.SpringArmComponent|SetbEnableCameraLag _springarm true)
      (Camera|SetFieldOfView _camtps 9e+01)
      (Transformation|SetRelativeLocation _camtps "0, 0, 0" false false)
      (Variables|/Script/Engine.CharacterMovementComponent|SetbOrientRotationToMovement _charactermovement true)
      (Variables|Default|SetbUseControllerRotationYaw false)
      (if (Variables|Default|GetReloading)
        _
        (else
          (Transformation|AttachComponentToComponent _m4 _mesh "RifleSocketMove" "KeepRelative" "KeepRelative" "KeepRelative" true)))
      (if _reloading
        _
        (else
          (Animation|StopAnimMontage "/Game/Assets/Characters/Swat/Animations/AM_Shooting.AM_Shooting")))
      (Utilities|IsValid _crosshairui
        (:Is%20Valid
          (Widget|SetVisibility _crosshairui "Hidden")
          (Default|ResetHitEffect _crosshairui))))))

(fn LandingDeceleration
  (Variables|/Script/Engine.MovementComponent|SetVelocity (Variables|Character|GetCharacterMovement) (* (Transformation|GetVelocity) 0.3)))

(fn LineTraceMuzzle
  (bind _camtps (Variables|Default|GetCamTPS))
  (Collision|LineTraceByChannel (Transformation|GetWorldLocation _camtps) (* (Math|Vector|GetForwardVector _camtps) 5e+04) "TraceTypeQuery1" false 0 "ForOneFrame"))

(fn ToggleFiremode
  (switch Utilities|FlowControl|Switch|SwitchonE_Firemode (Variables|Default|GetFiremode)
    (:NewEnumerator0
      (Variables|Default|SetFiremode "NewEnumerator1")
      (Audio|PlaySound2D "/Game/Assets/Sounds/Weapon/ToggleAuto.ToggleAuto" 1.0 1.0 0.0 0 0)
      (Variables|Default|SetFiremodeT "Auto"))
    (:NewEnumerator1
      (Variables|Default|SetFiremode "NewEnumerator0")
      (Audio|PlaySound2D "/Game/Assets/Sounds/Weapon/ToggleSemi.ToggleSemi" 1.0 1.0 0.0 0 0)
      (Variables|Default|SetFiremodeT "Semi-auto"))))

(fn RecoverSpread
  (params (DeltaTime :type Float%20%28double-precision%29))
  (Variables|Default|SetCurrentSpread (Math|Interpolation|FInterpTo (Variables|Default|GetCurrentSpread) (Variables|Default|GetMinSpread) DeltaTime (Variables|Default|GetSpreadRecoverSpeed))))

(fn FindGenerator
  (bind _generatordirection (Variables|Default|GetGeneratorDirection))
  (bind _generatordirection_2 (Variables|Default|GetGeneratorDirection))
  (bind _returnvalue (Transformation|GetWorldLocation _generatordirection))
  (Utilities|IsValid (Variables|Default|GetWaveManager%20Ref)
    (:Is%20Valid
      (Utilities|IsValid (Utilities|Array|Get(acopy) (Variables|/Game/Blueprints/BP_WaveManager.BP_WaveManager_C|GetGenerators (Variables|Default|GetWaveManager%20Ref)) (Variables|/Game/Blueprints/BP_WaveManager.BP_WaveManager_C|GetCurrentWave (Variables|Default|GetWaveManager%20Ref)))
        (:Is%20Valid
          (if (< (Math|Vector|VectorLength (- _returnvalue (Transformation|GetActorLocation (Utilities|Array|Get(acopy) (Variables|/Game/Blueprints/BP_WaveManager.BP_WaveManager_C|GetGenerators (Variables|Default|GetWaveManager%20Ref)) (Variables|/Game/Blueprints/BP_WaveManager.BP_WaveManager_C|GetCurrentWave (Variables|Default|GetWaveManager%20Ref)))))) 5e+02)
            (Rendering|SetVisibility _generatordirection_2 false false)
            (else
              (Transformation|SetWorldRotation _generatordirection (Math|Rotator|MakeRotator 0.0 0.0 (.yaw (Math|Rotator|FindLookatRotation _returnvalue (Transformation|GetActorLocation (Utilities|Array|Get(acopy) (Variables|/Game/Blueprints/BP_WaveManager.BP_WaveManager_C|GetGenerators (Variables|Default|GetWaveManager%20Ref)) (Variables|/Game/Blueprints/BP_WaveManager.BP_WaveManager_C|GetCurrentWave (Variables|Default|GetWaveManager%20Ref))))))) false false)
              (Rendering|SetVisibility _generatordirection_2 true false))))))
    (:Is%20Not%20Valid
      (bind _returnvalue_2 (Actor|GetActorOfClass "/Game/Blueprints/BP_WaveManager.BP_WaveManager_C"))
      (Variables|Default|SetWaveManager%20Ref _returnvalue_2))))

(fn GetCollision
  (return (Variables|Collision|GetCapsuleComponent)))

(fn KnockbackStrength
  (return 0.0))