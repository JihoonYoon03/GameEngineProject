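; BP_DroppedShell is a short-lived physics actor for a dropped shell.
; On BeginPlay it launches the Shell component along SpawnDirection scaled by SpawnImpulse, adds a randomized angular impulse for tumbling, and sets a brief lifespan so it cleans itself up.
; The component's hit event passes through a DoOnce, so the drop sound plays only at the first impact location.
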(event OnComponentHit(Shell)
  (params (HitComponent :type Primitive%20Component%20Object%20Reference) (OtherActor :type Actor%20Object%20Reference) (OtherComp :type Primitive%20Component%20Object%20Reference) (NormalImpulse :type Vector :default "0, 0, 0") (Hit :type Hit%20Result%20Structure%20%28by%20ref%29))
  (Utilities|FlowControl|DoOnce false
    (:Completed
      (Audio|PlaySoundatLocation "/Game/Assets/Sounds/Weapon/Bullet/ShellDropCue.ShellDropCue" (.location Hit) "0, 0, 0" 1.0 1.0 0.0 0 0 0 0))))

(event EventBeginPlay
  (bind _shell (Variables|Default|GetShell))
  (Physics|AddImpulse _shell (* (Variables|Default|GetSpawnDirection) (Variables|Default|GetSpawnImpulse)) "None" false)
  (Class|PrimitiveComponent|AddAngularImpulseinDegrees _shell (* (Math|Random|RandomUnitVector) (Math|Random|RandomFloatinRange 3e+02 9e+02)) "None" false)
  (Actor|SetLifeSpan 3.0))

(event Collision|EventActorBeginOverlap
  (params (OtherActor :type Actor%20Object%20Reference)))

(event EventTick
  (params (DeltaSeconds :type Float%20%28single-precision%29)))

(fn ConstructionScript)