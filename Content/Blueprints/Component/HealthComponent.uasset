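; HealthComponent is a component that tracks an owner's health and death state.
; InitialHP sets the maximum and fills current health to it.
; GetDamage subtracts a value, flags that a hit happened and marks the owner dead at zero or below.
; Tick recomputes the health ratio from current and maximum health every frame.
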(event EventBeginPlay)

(event EventTick
  (params (DeltaSeconds :type Float%20%28single-precision%29))
  (Variables|Default|SetHealthRatio (/ (Variables|Default|GetCurrentHealth) (Variables|Default|GetMaxHealth))))

(fn GetDamage
  (params (Value :type Float%20%28double-precision%29))
  (bind _output_get (Variables|Default|SetCurrentHealth (- (Variables|Default|GetCurrentHealth) Value)))
  (Variables|Default|SetGot%20Hit? true)
  (if (<= _output_get 0.0)
    (Variables|Default|SetIsDead? true)))

(fn InitialHP
  (params (HP :type Float%20%28double-precision%29))
  (bind _output_get (Variables|Default|SetMaxHealth HP))
  (Variables|Default|SetCurrentHealth _output_get))