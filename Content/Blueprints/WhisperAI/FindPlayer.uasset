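; Behavior tree task for the Whisper AI that sets the player as target and checks whether it has noticed them.
; It writes player pawn 0 and the Whisper's attack range to the Blackboard.
; It succeeds if the Whisper's health component reports a hit or the player is within a fixed distance, otherwise it fails.
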(event EventReceiveExecuteAI
  (params (OwnerController :type AI%20Controller%20Object%20Reference) (ControlledPawn :type Pawn%20Object%20Reference))
  (bind _returnvalue (Game|Player|GetPlayerPawn 0))
  (Class|BTFunctionLibrary|SetBlackboardValueasObject (Variables|Default|GetTarget%20Player%20Key) _returnvalue)
  (bind _asbp_whisper (Utilities|Casting|CastToBP_Whisper ControlledPawn)
    (:then
      (Class|BTFunctionLibrary|SetBlackboardValueasFloat (Variables|Default|GetAttack%20Range%20Key) (Variables|/Game/Blueprints/BP_Whisper.BP_Whisper_C|GetAttackRange _asbp_whisper)))
    (:CastFailed
      _))
  (AI|BehaviorTree|FinishExecute (or (Variables|/Game/Blueprints/Component/HealthComponent.HealthComponent_C|GetGot%20Hit? (Variables|/Game/Blueprints/BP_Whisper.BP_Whisper_C|GetHealthComponent _asbp_whisper)) (< (Math|Vector|Distance(Vector) (Transformation|GetActorLocation ControlledPawn) (Transformation|GetActorLocation _returnvalue)) 1e+03))))