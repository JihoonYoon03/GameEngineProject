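; Behavior tree service in WhisperAI that flags whether the AI pawn is close enough to attack its target.
; Each tick, it requests a collision component from the blackboard target through GetCollisionMessage.
; If valid, it compares the pawn's distance to that collision's closest point against the blackboard attack range, writing the CanAttack key.
; Measuring to the collision surface instead of the target's origin accounts for target size.
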(event EventReceiveTickAI
  (params (OwnerController :type AI%20Controller%20Object%20Reference) (ControlledPawn :type Pawn%20Object%20Reference) (DeltaSeconds :type Float%20%28single-precision%29))
  (bind _collision (Class|GetCollisionInterface|GetCollision(Message) (Class|BTFunctionLibrary|GetBlackboardValueasObject (Variables|Default|GetTarget%20Key))))
  (Utilities|IsValid _collision
    (:Is%20Valid
      (Class|BTFunctionLibrary|SetBlackboardValueasBool (Variables|Default|GetCanAttack%20Key) (<= (.ReturnValue (Collision|GetClosestPointonCollision _collision (Transformation|GetActorLocation ControlledPawn) "None")) (Class|BTFunctionLibrary|GetBlackboardValueasFloat (Variables|Default|GetAttack%20Range%20Key)))))))