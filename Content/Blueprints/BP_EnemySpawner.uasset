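; Enemy spawner actor that places BP_Whisper enemies at random navigable points around itself.
; SpawnEnemy retries FindSpawnPoint up to about 100 times, then spawns a Whisper with the given MainObjective, sets its speed and returns it.
; FindSpawnPoint picks a random horizontal offset between MinRadius and MaxRadius and projects it onto the navmesh with a tall vertical extent.
; The construction script sizes the Sphere component to MaxRadius.
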(event EventBeginPlay)

(event Collision|EventActorBeginOverlap
  (params (OtherActor :type Actor%20Object%20Reference)))

(event EventTick
  (params (DeltaSeconds :type Float%20%28single-precision%29)))

(fn ConstructionScript
  (Components|Sphere|SetSphereRadius (Variables|Default|GetSphere) (Variables|Default|GetMaxRadius) false))

(fn SpawnEnemy
  (params (MainObjective :type Actor%20Object%20Reference))
  (Utilities|FlowControl|ForLoopwithBreak 0 100
    (:LoopBody
      (bind (_found _projectedlocation) (CallFunction|FindSpawnPoint))
      (if _found
        (bind _returnvalue (Game|SpawnActorfromClass "/Game/Blueprints/BP_Whisper.BP_Whisper_C" (Math|Transform|MakeTransform _projectedlocation (Math|Random|RandomRotator false) "1.000000,1.000000,1.000000") "AdjustIfPossibleButAlwaysSpawn" "MultiplyWithRoot" 0 MainObjective 0))
        (Variables|/Game/Blueprints/BP_Whisper.BP_Whisper_C|SetMaxSpeed _returnvalue 2e+02)
        (return _returnvalue)))
    (:Completed
      (return 0))))

(fn FindSpawnPoint
  (bind _returnvalue (Transformation|GetActorLocation))
  (bind _returnvalue_2 (Math|Random|RandomUnitVector))
  (bind _maxradius (Variables|Default|GetMaxRadius))
  (bind _minradius (Variables|Default|GetMinRadius))
  (bind _returnvalue_3 (Class|KismetMathLibrary|VectorNormal2D _returnvalue_2 0.0001))
  (bind _returnvalue_4 (Math|Random|RandomFloatinRange _minradius _maxradius))
  (bind _returnvalue_5 (* _returnvalue_3 _returnvalue_4))
  (bind _returnvalue_6 (+ _returnvalue_5 _returnvalue))
  (bind (_projectedlocation _returnvalue_7) (AI|Navigation|ProjectPointtoNavigation _returnvalue_6 0 0 "50.000000,50.000000,100000.000000"))
  (return _returnvalue_7 _projectedlocation))