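; Whisper is an AI melee enemy with a health component, random idle growls and walk speed that eases down to its cap.
; Attack plays a random montage section whose notifies open the damage window for hand-collider overlaps.
; Damage from non-Whispers triggers a hit reaction and knockback, scaled by the causer's reported strength.
; On death, Tick halts AI and movement, ignores pawn collision, then broadcasts and destroys at a montage notify.
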(event OnComponentBeginOverlap(RHand)
  (params (OverlappedComponent :type Primitive%20Component%20Object%20Reference) (OtherActor :type Actor%20Object%20Reference) (OtherComp :type Primitive%20Component%20Object%20Reference) (OtherBodyIndex :type Integer) (bFromSweep :type Boolean) (SweepResult :type Hit%20Result%20Structure%20%28by%20ref%29))
  ;[0.15 0.15 0.15 0.5 50] Attack
  ;;[0.15 0.15 0.15 0.5 23] Attack Hit
  (if (Variables|Default|GetAttack?)
    (Game|Damage|ApplyDamage OtherActor (Variables|Default|GetBaseDamage) 0 self "/Game/Blueprints/Damage/Scratch.Scratch_C")))

(event OnComponentBeginOverlap(LHand)
  (params (OverlappedComponent :type Primitive%20Component%20Object%20Reference) (OtherActor :type Actor%20Object%20Reference) (OtherComp :type Primitive%20Component%20Object%20Reference) (OtherBodyIndex :type Integer) (bFromSweep :type Boolean) (SweepResult :type Hit%20Result%20Structure%20%28by%20ref%29))
  ;[0.15 0.15 0.15 0.5 50] Attack
  ;;[0.15 0.15 0.15 0.5 23] Attack Hit
  (if (Variables|Default|GetAttack?)
    (Game|Damage|ApplyDamage OtherActor (Variables|Default|GetBaseDamage) 0 self "/Game/Blueprints/Damage/Scratch.Scratch_C")))

(event Custom|Attack
  ;[0.15 0.15 0.15 0.5 50] Attack
  (if (not (Variables|/Game/Blueprints/Component/HealthComponent.HealthComponent_C|GetIsDead? (Variables|Default|GetHealthComponent)))
    (Utilities|FlowControl|DoOnce false :!label _label
      (:Completed
        (bind _notifyname (Animation|Montage|PlayMontage (Variables|Character|GetMesh) "/Game/Assets/Characters/Creature/Whisper/Animations/WhisperAttack.WhisperAttack" 1.0 0.0 (Utilities|String|StringToName (Utilities|String|ToString(Integer) (Math|Random|RandomIntegerinRange 1 3))))
          (:OnCompleted
            (goto _label Reset))
          (:OnInterrupted
            (goto _label Reset))
          (:OnNotifyBegin
            (switch name _notifyname
              (:Enable
                (Variables|Default|SetAttack? true)
                (Audio|PlaySoundatLocation "/Game/Assets/Sounds/Enemy/Whisper/WhisperAttackCue.WhisperAttackCue" "0, 0, 0" "0, 0, 0" 1.0 1.0 0.0 0 0 0 0))
              (:Disable
                (Variables|Default|SetAttack? false)))))))))

(event EventBeginPlay
  (Variables|Default|SetGrowlRandomTime (Math|Random|RandomFloatinRange 3.0 7.0))
  (Default|InitialHP (Variables|Default|GetHealthComponent) 2e+02))

(event Collision|EventActorBeginOverlap
  (params (OtherActor :type Actor%20Object%20Reference)))

(event EventTick
  (params (DeltaSeconds :type Float%20%28single-precision%29))
  (bind _self self)
  (bind _returnvalue (AI|GetAIController _self))
  (if (Variables|/Game/Blueprints/Component/HealthComponent.HealthComponent_C|GetIsDead? (Variables|Default|GetHealthComponent))
    ;[0.15 0.15 0.15 0.5 32] Dead
    (Utilities|FlowControl|DoOnce false
      (:Completed
        (AI|Navigation|StopMovement _returnvalue)
        (AI|Logic|StopLogic (Variables|/Script/AIModule.AIController|GetBrainComponent _returnvalue) "Dead")
        (Components|Movement|StopMovementImmediately (Variables|Character|GetCharacterMovement))
        (Collision|SetCollisionResponsetoChannel (Variables|Collision|GetCapsuleComponent) "ECC_Pawn" "ECR_Ignore")
        (Animation|Montage|PlayMontage (Variables|Character|GetMesh) "/Game/Assets/Characters/Creature/Whisper/Animations/WhisperDeath.WhisperDeath"
          (:OnNotifyBegin
            (Default|CallOnEnemyDeath)
            (Actor|DestroyActor)))))
    (else
      (Variables|Default|SetCurrentMainObject 0)
      (CallFunction|WalkDeceleration DeltaSeconds)
      (Variables|Default|SetCurSpeed (Math|Vector|VectorLength (Transformation|GetVelocity)))
      ;[0.15 0.15 0.15 0.5 32] Random Sound
      (if (< (Variables|Default|GetGrowlRandomTime) (Variables|Default|GetGrowlDeltaTime))
        (Audio|PlaySoundatLocation "/Game/Assets/Sounds/Enemy/Whisper/WhisperIdleCue.WhisperIdleCue" (Transformation|GetActorLocation) "0, 0, 0" 1.0 1.0 0.0 0 0 0 0)
        (Variables|Default|SetGrowlRandomTime (Math|Random|RandomFloatinRange 3.0 7.0))
        (Variables|Default|SetGrowlDeltaTime 0.0)
        (else
          (Variables|Default|SetGrowlDeltaTime (+ (Variables|Default|GetGrowlDeltaTime) DeltaSeconds)))))))

(event Game|Damage|EventAnyDamage
  (params (Damage :type Float%20%28single-precision%29) (DamageType :type Damage%20Type%20Object%20Reference) (InstigatedBy :type Controller%20Object%20Reference) (DamageCauser :type Actor%20Object%20Reference))
  ;[0.15 0.15 0.15 0.5 32] Damaged
  (if (not (Variables|/Game/Blueprints/Component/HealthComponent.HealthComponent_C|GetIsDead? (Variables|Default|GetHealthComponent)))
    (Utilities|Casting|CastToBP_Whisper DamageCauser
      (:CastFailed
        (Default|GetDamage (Variables|Default|GetHealthComponent) Damage)
        (bind _strength (Class|KnockbackInteface|KnockbackStrength(Message) DamageCauser))
        (CallFunction|ApplyKnockback DamageCauser _strength)
        (Variables|Default|SetHit? true)
        (Animation|Montage|PlayMontage (Variables|Character|GetMesh) "/Game/Assets/Characters/Creature/Whisper/Animations/WhisperHitReact.WhisperHitReact" 1.0 0.0 (Utilities|String|StringToName (Utilities|String|ToString(Integer) (Math|Random|RandomIntegerinRange 1 2)))
          (:OnCompleted
            _)
          (:OnBlendOut
            _))
        (Variables|Default|SetHit? false)))))

(event EventApplyKnockback
  (params (Damage%20Causer :type Actor%20Object%20Reference) (Strength :type Float%20%28double-precision%29))
  ;[0.15 0.15 0.15 0.5 32] Damaged
  ;;[0.15 0.15 0.15 0.5] Knockback
  (Character|LaunchCharacter (+ (* Strength (Math|Vector|Normalize (- (Transformation|GetActorLocation) (Transformation|GetActorLocation Damage%20Causer)))) "0.000000,0.000000,20.000000") false false))

(fn ConstructionScript)

(fn WalkDeceleration
  (params (DeltaTime :type Float%20%28double-precision%29))
  (bind _charactermovement (Variables|Character|GetCharacterMovement))
  (bind _maxspeed (Variables|Default|GetMaxSpeed))
  ;[0.15 0.15 0.15 0.5] Set Max Walk Speed with Interpolation
  (if (< _maxspeed (Variables|/Script/Engine.CharacterMovementComponent|GetMaxWalkSpeed _charactermovement))
    (Variables|/Script/Engine.CharacterMovementComponent|SetMaxWalkSpeed _charactermovement (Math|Interpolation|FInterpTo (Variables|/Script/Engine.CharacterMovementComponent|GetMaxWalkSpeed _charactermovement) _maxspeed DeltaTime 8.0))))

(fn GetCollision
  (return (Variables|Collision|GetCapsuleComponent)))

(fn KnockbackStrength
  (return 5e+01))