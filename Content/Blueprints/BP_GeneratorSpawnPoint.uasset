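; Generator spawn point actor that spawns BP_Whisper enemies and previews an array of spawn points in the editor.
; The construction script grows SpawnPoints to at least SpawnLimit and adds an arrow mesh at each point, which BeginPlay destroys.
; SpawnEnemy ignores those points, spawning a randomly rotated Whisper at the actor's location, as its random XY offset range is zero.
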(event EventBeginPlay
  (for _array_element (Variables|Default|GetArrows)
    (Components|DestroyComponent _array_element)))

(event Collision|EventActorBeginOverlap
  (params (OtherActor :type Actor%20Object%20Reference)))

(event EventTick
  (params (DeltaSeconds :type Float%20%28single-precision%29)))

(fn ConstructionScript
  (bind _spawnlimit (Variables|Default|GetSpawnLimit))
  (bind _spawnpoints (Variables|Default|GetSpawnPoints))
  (if (> _spawnlimit (Utilities|Array|Length (Variables|Default|GetSpawnPoints)))
    (Utilities|Array|Resize _spawnpoints _spawnlimit))
  (for _array_element _spawnpoints
    (bind _returnvalue (AddComponent|AddStaticMeshComponent false (Math|Transform|MakeTransform _array_element "-90.000000,0.000000,0.000000" "20.000000,4.000000,4.000000")))
    (Utilities|Array|Add (Variables|Default|GetArrows) _returnvalue)))

(fn SpawnEnemy
  (bind _returnvalue (Math|Random|RandomUnitVector))
  (bind _returnvalue_2 (Math|Random|RandomFloatinRange 0.0 0.0))
  (bind _returnvalue_3 (* _returnvalue _returnvalue_2))
  (bind _returnvalue_4 (Game|SpawnActorfromClass "/Game/Blueprints/BP_Whisper.BP_Whisper_C" (Math|Transform|MakeTransform (+ (Transformation|GetActorLocation) (Math|Vector|MakeVector (.x _returnvalue_3) (.y _returnvalue_3) 0.0)) (Math|Random|RandomRotator false) "1.000000,1.000000,1.000000") "AdjustIfPossibleButAlwaysSpawn" "MultiplyWithRoot" 0 0))
  (return _returnvalue_4))